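; BP_GhostPlayerController is the player controller for the Ghost game, switching the player to UI control when a level ends or fails.
; On BeginPlay it casts the game mode to BP_GhostGamemode and binds handlers to its restart-level and level-end events.
; Both handlers disable input, set UI-only input mode focused on the player widget with the mouse locked, and show the cursor.
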(event `self.ReceiveBeginPlay`
  (bind _output_get (set `self.ReferenceToGameMode` (cast `/Game/Ghost/BP_GhostGamemode` (`GameplayStatics.GetGameMode`) :!pure true)))
  (add `/Game/Ghost/BP_GhostGamemode.RestartLevel` _output_get (delegate `Handle Level Failed`))
  (add `/Game/Ghost/BP_GhostGamemode.LevelEnd` _output_get (delegate `Handle Level End`)))

(event `Handle Level Failed`
  (`self.DisableInputAndUseUI`))

(event `Handle Level End`
  (`self.DisableInputAndUseUI`))

(event `DisableInputAndUseUI`
  (`self.DisableInput` self)
  (`WidgetBlueprintLibrary.SetInputMode_UIOnlyEx` self (`self.PlayerWidget`) "LockAlways")
  (set `self.bShowMouseCursor` true))

(fn `UserConstructionScript`)