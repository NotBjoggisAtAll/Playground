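; BP_Spikes is a spikes actor that detects overlaps from the player character and ghosts, currently only printing which one touched it.
; On BeginPlay it casts the first player controller's pawn to MyCharacter and caches the reference.
; The static mesh's begin-overlap event compares the other actor to that reference, then checks for an exact BP_Ghost class match, printing a label for each.
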(event `self.ReceiveBeginPlay`
  (bind _asmy_character (cast `MyCharacter` (`Controller.K2_GetPawn` (`GameplayStatics.GetPlayerController` 0))))
  (set `self.Reference To MyCharacter` _asmy_character))

(event `self.StaticMesh.OnComponentBeginOverlap`
  (params (OverlappedComponent :type "PrimitiveComponent Object Reference") (OtherActor :type "Actor Object Reference") (OtherComp :type "PrimitiveComponent Object Reference") (OtherBodyIndex :type Integer) (bFromSweep :type Boolean) (SweepResult :type "HitResult Structure (by ref)"))
  (if (== OtherActor (`self.Reference To MyCharacter`))
    (`KismetSystemLibrary.PrintString` "Player")
    (elif (== (`GameplayStatics.GetObjectClass` OtherActor) "/Game/Ghost/BP_Ghost.BP_Ghost_C")
      (`KismetSystemLibrary.PrintString` "Ghost"))))

(fn `UserConstructionScript`)