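; BP_Spikes is a button-driven spike hazard that restarts the level when its moveable mesh overlaps the player or a clone.
; It inherits button press and release handling from its parent and plays the same spike sound at the mesh whenever it opens or closes.
; An overlap with the cached player character or a BP_Clone plays a crushing sound and calls the level restart on BP_GameMode.
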(event `OnOpen`
  (`GameplayStatics.PlaySoundAtLocation` "/Game/Sounds/SpikesDown.SpikesDown" (`SceneComponent.K2_GetComponentLocation` (`self.MoveableMesh`)) (struct) 1.0 1.0 0.0 null null null :!label _label))

(event `OnClosed`
  (goto _label))

(event `self.OnButtonsPressed`
  (`parent.OnButtonsPressed`))

(event `self.OnButtonsReleased`
  (`parent.OnButtonsReleased`))

(event `self.ReceiveBeginPlay`
  (`parent.ReceiveBeginPlay`)
  (set `self.Reference To MyCharacter` (cast `MyCharacter` (`GameplayStatics.GetPlayerPawn` 0) :!pure true))
  (add `self.OnOpenDelegate` (delegate `HandleOnOpen`))
  (add `self.OnClosedDelegate` (delegate `HandleOnClosed`)))

(event `HandleOnOpen`
  (`self.OnOpen`))

(event `HandleOnClosed`
  (`self.OnClosed`))

(event `self.MoveableMesh.OnComponentBeginOverlap`
  (params (OverlappedComponent :type "PrimitiveComponent Object Reference") (OtherActor :type "Actor Object Reference") (OtherComp :type "PrimitiveComponent Object Reference") (OtherBodyIndex :type Integer) (bFromSweep :type Boolean) (SweepResult :type "HitResult Structure (by ref)"))
  (if (== OtherActor (`self.Reference To MyCharacter`))
    (`|ExecutionSequence` :!label _label_2
      (:`then_0`
        (`GameplayStatics.PlaySoundAtLocation` "/Game/Sounds/crushingsound.crushingsound" SweepResult_Location (struct) 1.0 1.0 0.0 null null null))
      (:`then_1`
        (`/Game/Blueprints/BP_GameMode.RestartLevel` (cast `/Game/Blueprints/BP_GameMode` (`GameplayStatics.GetGameMode`) :!pure true))))
    (elif (== (`GameplayStatics.GetObjectClass` OtherActor) "/Game/Blueprints/BP_Clone.BP_Clone_C")
      (goto _label_2))))

(fn `UserConstructionScript`)