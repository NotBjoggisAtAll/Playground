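; Game mode Blueprint that starts looping background music and gives feedback when a level is failed or won.
; On BeginPlay it binds handlers to the RestartLevel and LevelEnd event dispatchers.
; Failure only prints a red restart message, with no reload logic here.
; A win prints a green message, plays a cheer and triggers LaunchShell on every TS_FireworksLauncher in the level.
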(event `self.ReceiveBeginPlay`
  (add `self.RestartLevel` (delegate `RestartLevel_Event`))
  (add `self.LevelEnd` (delegate `LevelEnd_Event`))
  (`GameplayStatics.PlaySound2D` "/Game/ImportedContent/MegaGameMusicCollection/CasualGameMusicPack/Cues/Casual_Theme__2__Looped__Cue.Casual_Theme__2__Looped__Cue" 0.7 1.0 0.0 null null))

(event `RestartLevel_Event`
  (`KismetSystemLibrary.PrintString` "LEVEL FAILED. RESTART" true true (struct :`R` 1.0 :`B` 0.015156 :`A` 1.0) 10.0))

(event `LevelEnd_Event`
  (`KismetSystemLibrary.PrintString` "Level Won" true true (struct :`R` 0.087081 :`G` 1.0 :`A` 1.0) 10.0)
  (`GameplayStatics.PlaySound2D` "/Game/Sounds/yaaay.yaaay" 0.4 1.0 0.0 null null)
  (bind _outactors (`GameplayStatics.GetAllActorsOfClass` "/Game/ImportedContent/TS_Fireworks/Blueprints/TS_FireworksLauncher.TS_FireworksLauncher_C"))
  (for _array_element _outactors
    (`/Game/ImportedContent/TS_Fireworks/Blueprints/TS_FireworksLauncher.LaunchShell` _array_element)))

(fn `UserConstructionScript`)