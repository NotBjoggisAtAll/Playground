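; BP_LevelEndTrigger is a trigger actor that ends the level when the player enters it.
; On BeginPlay it caches the first player pawn as BP_Character and the game mode as BP_GameMode.
; When an overlapping actor matches the cached player, it calls CallLevelEnd on the game mode, which handles the level end itself.
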(event `self.ReceiveBeginPlay`
  (set `self.ReferenceToPlayer` (cast `/Game/Blueprints/BP_Character` (`GameplayStatics.GetPlayerPawn` 0) :!pure true))
  (set `self.ReferenceToGameMode` (cast `/Game/Blueprints/BP_GameMode` (`GameplayStatics.GetGameMode`) :!pure true)))

(event `self.ReceiveActorBeginOverlap`
  (params (OtherActor :type "Actor Object Reference"))
  (if (== OtherActor (`self.ReferenceToPlayer`))
    (`/Game/Blueprints/BP_GameMode.LevelEnd` (`self.ReferenceToGameMode`))))

(fn `UserConstructionScript`)